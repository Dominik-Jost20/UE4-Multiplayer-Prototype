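; Plane actor that flies a randomized straight route across the map at constant speed and fixed height.
; On BeginPlay, the authority picks a start on a map-sized circle around the origin and a roughly opposite end, randomly deviated by yaw.
; It also sets up the spring arm, faces the plane along the path and derives its lifespan from map size and speed.
; Tick, without an authority check, moves it toward the end point.
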(event EventBeginPlay
  (bind _springarm (Variables|Default|GetSpringArm))
  (Networking|SwitchHasAuthority
    (:Authority
      (Variables|/Script/Engine.SpringArmComponent|SetTargetArmLength _springarm 2e+02)
      (Variables|/Script/Engine.SpringArmComponent|SetTargetOffset _springarm "0, 0,100.000000")
      (Actor|SetLifeSpan (/ (Variables|Default|GetMapSize) (Variables|Default|GetFlightSpeed)))
      (bind _output_get (Variables|Default|SetCenterOffset (Math|Vector|Normalize (Math|Vector|MakeVector (Math|Trig|Cos(Degrees) (Math|Random|RandomFloatinRange -1.8e+02 1.8e+02)) (Math|Trig|Sin(Degrees) (Math|Random|RandomFloatinRange -1.8e+02 1.8e+02)) 0.0))))
      (Variables|Default|SetFlightPathStart (* _output_get (/ (Variables|Default|GetMapSize) 2.0)))
      (Variables|Default|SetFlightPathEnd (* (Math|Vector|RotateVector (* (Variables|Default|GetCenterOffset) -1.0) (Math|Rotator|MakeRotator 0.0 0.0 (Math|Random|RandomFloatinRange -15.0 15.0))) (/ (Variables|Default|GetMapSize) 2.0)))
      (Transformation|SetActorRotation (Math|Conversions|RotationFromXVector (- (Variables|Default|GetFlightPathEnd) (Variables|Default|GetFlightPathStart))))
      (Transformation|SetActorRelativeLocation (Variables|Default|GetFlightPathStart)))))

(event EventTick
  (params (DeltaSeconds :type Float%20%28single-precision%29))
  (bind _returnvalue (Transformation|GetActorLocation))
  (bind _flightpathend (Variables|Default|GetFlightPathEnd))
  (bind _flightspeed (Variables|Default|GetFlightSpeed))
  (bind _returnvalue_2 (Math|Interpolation|VInterptoConstant _returnvalue _flightpathend DeltaSeconds _flightspeed))
  (bind (_x _y) (Math|Vector|BreakVector _returnvalue_2))
  (Transformation|SetActorLocation (Math|Vector|MakeVector _x _y (Variables|Default|GetFlyHight)) false false))

(fn ConstructionScript)