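; Weapon pickup Blueprint that offers a weapon to characters and carries its clip and spare ammo counts.
; On BeginPlay the authority fills both ammo counts from the weapon class defaults, unless a player dropped it, so dropped weapons keep their ammo.
; Pickup sphere events set the pickup as the character's current weapon pickup on entry and clear it on exit only if it is still current.
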(event EventBeginPlay
  (bind _weapontogive (Variables|Default|GetWeaponToGive))
  (bind (_damage _weaponname _currentammo _currentspareammo) (Utilities|GetClassDefaults _weapontogive))
  ;[1 1 1] remember ammo amounts if player dropped weapon
  (Networking|SwitchHasAuthority
    (:Authority
      (if (not (Variables|Default|GetDroppedByPlayer?))
        (Variables|Default|SetCurrentAmmoInClip _currentammo)
        (Variables|Default|SetCurrentSpareAmmo _currentspareammo)))))

(event EventPickupSphereEntered
  (params (Character :type BR%20Character%20Object%20Reference))
  ;[1 1 1] set player pickup
  (Variables|/Game/FirstPersonBP/Blueprints/Brcharacter.BRCharacter_C|SetCurrentWeaponPickup Character self))

(event EventPickupSphereLeft
  (params (Character :type BR%20Character%20Object%20Reference))
  ;[1 1 1] unset player pickup
  (if (== (Variables|/Game/FirstPersonBP/Blueprints/Brcharacter.BRCharacter_C|GetCurrentWeaponPickup Character) self)
    (Variables|/Game/FirstPersonBP/Blueprints/Brcharacter.BRCharacter_C|SetCurrentWeaponPickup Character 0)))

(fn ConstructionScript
  (|CallParentFunction))