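; BP_HealthPickup is a pickup that adjusts a character's health through the PickupSphereLeft event.
; On authority only, it checks that Health is below MaxHealth, then passes the negated HealthToGive to the character's ModifyHealth.
; It then prints the resulting health and destroys itself, staying in place when the character is already at full health.
; The construction script only calls its parent.
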(event EventPickupSphereLeft
  (params (Character :type BR%20Character%20Object%20Reference))
  (Networking|SwitchHasAuthority
    (:Authority
      (if (< (Variables|/Game/FirstPersonBP/Blueprints/Brcharacter.BRCharacter_C|GetHealth Character) (Variables|/Game/FirstPersonBP/Blueprints/Brcharacter.BRCharacter_C|GetMax%20Health Character))
        (Default|ModifyHealth Character (* (Variables|Default|GetHealthToGive) -1.0))
        (Development|PrintString (Utilities|String|ToString(Float) (Variables|/Game/FirstPersonBP/Blueprints/Brcharacter.BRCharacter_C|GetHealth Character)))
        (Actor|DestroyActor)))))

(fn ConstructionScript
  (|CallParentFunction))